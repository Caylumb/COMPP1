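; OrbitalCameraPawn is a camera pawn that orbits a selected target and issues commands to the player ship.
; It moves to CameraTarget on selection and every tick, with right-drag rotation while ShipMoveToggle is off and mouse-wheel zoom along the camera's local X.
; Enter makes the target the ship's orbit target, and Space flags that target destroyed if it is a PlanetoidDynamic the ship orbits.
; The PauseGame input opens the pause menu.
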(event EventTick
  (params (DeltaSeconds :type Float%20%28single-precision%29))
  (Utilities|IsValid (Variables|Default|GetCameraTarget)
    (:Is%20Valid
      (Transformation|SetActorLocation (Transformation|GetActorLocation (Variables|Default|GetCameraTarget)) false false))))

(event EventCameraSelect
  (params (TargetObject :type Actor%20Object%20Reference))
  (Variables|Default|SetCameraTarget TargetObject)
  (Transformation|SetActorLocation (Transformation|GetActorLocation (Variables|Default|GetCameraTarget)) false false))

(event Input|ActionEvents|InputActionPauseGame
  (params (Key :type Key%20Structure :default "None"))
  (:Pressed
    (if (not (Variables|Default|GetisPaused))
      (bind _returnvalue (UserInterface|CreateWidget "/Game/Blueprints/Hud/PauseMenu.PauseMenu_C"))
      (UserInterface|Viewport|AddtoViewport _returnvalue 0))))

(event Input|MouseEvents|MouseX
  (params (AxisValue :type Float%20%28single-precision%29))
  (if (and (not (Variables|Default|GetShipMoveToggle)) (Variables|Default|GetRMBDown))
    (Pawn|Input|AddControllerYawInput (* AxisValue 2.0))))

(event Input|MouseEvents|MouseY
  (params (AxisValue :type Float%20%28single-precision%29))
  (if (and (not (Variables|Default|GetShipMoveToggle)) (Variables|Default|GetRMBDown))
    (Pawn|Input|AddControllerPitchInput (* (* AxisValue 2.0) -1.0))))

(event Input|KeyboardEvents|Enter
  (params (Key :type Key%20Structure :default "None"))
  (:Pressed
    (if (!= (Variables|Default|GetCameraTarget) (Variables|Default|GetPlayerShip))
      (Variables|/Game/PlayerShip/PlayerShip.PlayerShip_C|SetShipOrbitTarget (Variables|Default|GetPlayerShip) (Variables|Default|GetCameraTarget)))))

(event Input|MouseEvents|RightMouseButton
  (params (Key :type Key%20Structure :default "None"))
  (:Pressed
    (Variables|Default|SetRMBDown true)
    (Pawn|SetControlRotation (Game|GetPlayerController 0) (Pawn|GetControlRotation :!class /Script/Engine.Pawn)))
  (:Released
    (Variables|Default|SetRMBDown false)))

(event Input|KeyboardEvents|SpaceBar
  (params (Key :type Key%20Structure :default "None"))
  (bind _cameratarget (Variables|Default|GetCameraTarget))
  (:Pressed
    (Utilities|IsValid (Variables|Default|GetCameraTarget)
      (:Is%20Valid
        (if (and (== (Utilities|GetClass _cameratarget) "/Game/Planetoid/PlanetoidDynamic.PlanetoidDynamic_C") (== _cameratarget (Variables|/Game/PlayerShip/PlayerShip.PlayerShip_C|GetShipOrbitTarget (Variables|Default|GetPlayerShip))))
          (bind _asplanetoid_dynamic (Utilities|Casting|CastToPlanetoidDynamic (Variables|Default|GetCameraTarget)))
          (Variables|/Game/Planetoid/PlanetoidDynamic.PlanetoidDynamic_C|SetisDestroyed _asplanetoid_dynamic true))))))

(event Input|MouseEvents|MouseWheelUp
  (params (Key :type Key%20Structure :default "None"))
  (bind _camera (Variables|Default|GetCamera))
  (:Pressed
    (Transformation|AddLocalOffset _camera (Math|Vector|MakeVector 5e+01 0.0 0.0) false false)
    (Variables|Default|SetDistance (.X (Math|Vector|BreakVector (Variables|/Script/Engine.SceneComponent|GetRelativeLocation _camera))))))

(event Input|MouseEvents|MouseWheelDown
  (params (Key :type Key%20Structure :default "None"))
  (bind _camera (Variables|Default|GetCamera))
  (:Pressed
    (Transformation|AddLocalOffset _camera (Math|Vector|MakeVector -5e+01 0.0 0.0) false false)
    (Variables|Default|SetDistance (.X (Math|Vector|BreakVector (Variables|/Script/Engine.SceneComponent|GetRelativeLocation _camera))))))

(fn ConstructionScript)